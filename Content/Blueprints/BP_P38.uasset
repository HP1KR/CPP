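; BP_P38 is a player-controllable P-38 aircraft actor that flies forward at a constant speed.
; Tick spins the left and right propeller components and offsets the actor along its local X axis, scaled by delta time without sweeping for collision.
; BeginPlay enables input from the first player controller, and the Roll and Pitch axes rotate the actor locally at RotationSpeed, also frame-rate independent.
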(event Collision|EventActorBeginOverlap
  (params (OtherActor :type Actor%20Object%20Reference)))

(event EventTick
  (params (DeltaSeconds :type Float%20%28single-precision%29))
  (Transformation|AddLocalRotation (Variables|Default|GetRightPropeller) (Math|Rotator|MakeRotator (* (Utilities|Time|GetWorldDeltaSeconds) 1e+03) 0.0 0.0) false false)
  (Transformation|AddLocalRotation (Variables|Default|GetLeftPropeller) (Math|Rotator|MakeRotator (* (Utilities|Time|GetWorldDeltaSeconds) 1e+03) 0.0 0.0) false false)
  (Transformation|AddActorLocalOffset (Math|Vector|MakeVector (* (Utilities|Time|GetWorldDeltaSeconds) 1e+02) 0.0 0.0) false false))

(event EventBeginPlay
  (Input|EnableInput (Game|GetPlayerController 0)))

(event Input|AxisEvents|InputAxisRoll
  (params (AxisValue :type Float%20%28single-precision%29))
  (Transformation|AddActorLocalRotation (Math|Rotator|MakeRotator (* AxisValue (Variables|Default|GetRotationSpeed) (Utilities|Time|GetWorldDeltaSeconds)) 0.0 0.0) false false))

(event Input|AxisEvents|InputAxisPitch
  (params (AxisValue :type Float%20%28single-precision%29))
  (Transformation|AddActorLocalRotation (Math|Rotator|MakeRotator 0.0 (* AxisValue (Variables|Default|GetRotationSpeed) (Utilities|Time|GetWorldDeltaSeconds)) 0.0) false false))

(fn ConstructionScript)