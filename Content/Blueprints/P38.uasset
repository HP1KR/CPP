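; P38 is an aircraft Blueprint with two propellers that animates a simple straight flight.
; Every Tick spins the left and right propeller components around their local roll axis and moves the root component along the world forward axis.
; Both motions are scaled by world delta seconds for frame-rate independence, with no input, collision response or construction logic.
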(event EventBeginPlay)

(event Collision|EventActorBeginOverlap
  (params (OtherActor :type Actor%20Object%20Reference)))

(event EventTick
  (params (DeltaSeconds :type Float%20%28single-precision%29))
  (Transformation|AddLocalRotation (Variables|Default|GetRightPropeller) (Math|Rotator|MakeRotator (* (Utilities|Time|GetWorldDeltaSeconds) 1e+03) 0.0 0.0) false false)
  (Transformation|AddLocalRotation (Variables|Default|GetLeftPropeller) (Math|Rotator|MakeRotator (* (Utilities|Time|GetWorldDeltaSeconds) 1e+03) 0.0 0.0) false false)
  (Class|SceneComponent|AddWorldTransform (Variables|Default|GetDefaultSceneRoot) (Math|Transform|MakeTransform (* (Class|KismetMathLibrary|VectorForward) (* (Utilities|Time|GetWorldDeltaSeconds) 1e+02)) "0, 0, 0" "1,1,1") false false))

(fn ConstructionScript)