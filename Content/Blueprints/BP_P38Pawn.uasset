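; BP_P38Pawn is a simple flyable P-38 aircraft pawn that enables input from the first player controller on BeginPlay.
; Each tick it spins the left and right propellers and moves the actor forward along its local X axis at MoveSpeed, without sweeping for collision.
; Roll and Pitch axis inputs rotate the actor locally, scaled by RotationSpeed and frame delta time, so steering changes the direction of flight.
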(event Collision|EventActorBeginOverlap
  (params (OtherActor :type Actor%20Object%20Reference)))

(event EventTick
  (params (DeltaSeconds :type Float%20%28single-precision%29))
  ;[1 1 1] Right Propeller Rotate
  (Transformation|AddLocalRotation (Variables|Default|GetRightPropeller) (Math|Rotator|MakeRotator (* (Utilities|Time|GetWorldDeltaSeconds) 1e+03) 0.0 0.0) false false)
  ;[1 1 1] Left Propeller Rotate
  (Transformation|AddLocalRotation (Variables|Default|GetLeftPropeller) (Math|Rotator|MakeRotator (* (Utilities|Time|GetWorldDeltaSeconds) 1e+03) 0.0 0.0) false false)
  ;[1 1 1] Move Forward
  (Transformation|AddActorLocalOffset (Math|Vector|MakeVector (* (Utilities|Time|GetWorldDeltaSeconds) (Variables|Default|GetMoveSpeed)) 0.0 0.0) false false))

(event EventBeginPlay
  (Input|EnableInput (Game|GetPlayerController 0)))

(event Input|AxisEvents|InputAxisRoll
  (params (AxisValue :type Float%20%28single-precision%29))
  ;[1 1 1] Roll
  (Transformation|AddActorLocalRotation (Math|Rotator|MakeRotator (* AxisValue (Variables|Default|GetRotationSpeed) (Utilities|Time|GetWorldDeltaSeconds)) 0.0 0.0) false false))

(event Input|AxisEvents|InputAxisPitch
  (params (AxisValue :type Float%20%28single-precision%29))
  ;[1 1 1] Pitch
  (Transformation|AddActorLocalRotation (Math|Rotator|MakeRotator 0.0 (* AxisValue (Variables|Default|GetRotationSpeed) (Utilities|Time|GetWorldDeltaSeconds)) 0.0) false false))

(fn ConstructionScript)